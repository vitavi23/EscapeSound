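; Animation notify that plays walking footstep sounds matched to the surface under the animated character.
; On notify, a Visibility line trace runs 200 units down along the owner's up vector, with timed debug drawing enabled.
; The hit's physical surface selects a walk sound cue per material, with concrete as the fallback.
; Sounds play at the world origin rather than the hit or owner location.
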(fn `Received_Notify`
  (params (MeshComp :type "SkeletalMeshComponent Object Reference") (Animation :type "AnimSequenceBase Object Reference") (EventReference :type "AnimNotifyEventReference Structure (by ref)"))
  (returns (ReturnValue :type Boolean))
  (bind _returnvalue (`ActorComponent.GetOwner` MeshComp))
  (bind _returnvalue_2 (`Actor.K2_GetActorLocation` _returnvalue))
  (bind _outhit (`KismetSystemLibrary.LineTraceSingle` :`Start` _returnvalue_2 :`End` (+ _returnvalue_2 (* (`Actor.GetActorUpVector` _returnvalue) -200.0)) :`TraceChannel` "TraceTypeQuery1" :`DrawDebugType` "ForDuration"))
  (if true
    (switch `EPhysicalSurface` (`GameplayStatics.GetSurfaceType` _outhit)
      (:`SurfaceType_Default`
        (`GameplayStatics.PlaySoundAtLocation` "/Game/Audio/Footsteps/Walk/Concrete/SC_Concrete_Walk.SC_Concrete_Walk" (0.0 0.0 0.0) (struct) 1.0 1.0 0.0 null null null null :!label _label))
      (:`SurfaceType1`
        (goto _label))
      (:`SurfaceType2`
        (`GameplayStatics.PlaySoundAtLocation` "/Game/Audio/Footsteps/Walk/Woodplank/SC_Woodplank_Walk.SC_Woodplank_Walk" (0.0 0.0 0.0) (struct) 1.0 1.0 0.0 null null null null))
      (:`SurfaceType3`
        (`GameplayStatics.PlaySoundAtLocation` "/Game/Audio/Footsteps/Walk/Metal/SC_Metal_Walk.SC_Metal_Walk" (0.0 0.0 0.0) (struct) 1.0 1.0 0.0 null null null null))
      (:`SurfaceType4`
        (`GameplayStatics.PlaySoundAtLocation` "/Game/Audio/Footsteps/Walk/Parquet/SC_Parquet_Walk.SC_Parquet_Walk" (0.0 0.0 0.0) (struct) 1.0 1.0 0.0 null null null null))
      (:`SurfaceType5`
        (`GameplayStatics.PlaySoundAtLocation` "/Game/Audio/Footsteps/Walk/Sand/SC_Sand_Walk.SC_Sand_Walk" (0.0 0.0 0.0) (struct) 1.0 1.0 0.0 null null null null))
      (:`SurfaceType6`
        (`GameplayStatics.PlaySoundAtLocation` "/Game/Audio/Footsteps/Walk/Stone/SC_Stone_Walk.SC_Stone_Walk" (0.0 0.0 0.0) (struct) 1.0 1.0 0.0 null null null null)))
    (return false)))